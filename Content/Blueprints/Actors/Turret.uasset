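; Turret actor that fires homing-target projectiles at a DHeroCharacter inside its AttackRadius.
; On overlap it fires immediately and starts a two-second looping timer, spawning a Turret_Projectile at ProjectileSpawn with the hero's capsule as ProjectileTarget.
; Leaving the radius clears the timer by re-setting it with zero time and resets the DoOnce that guards against double firing on re-entry.
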(event OnComponentBeginOverlap(AttackRadius)
  (params (OverlappedComponent :type Primitive%20Component%20Object%20Reference) (OtherActor :type Actor%20Object%20Reference) (OtherComp :type Primitive%20Component%20Object%20Reference) (OtherBodyIndex :type Integer) (bFromSweep :type Boolean) (SweepResult :type Hit%20Result%20Structure%20%28by%20ref%29))
  ;[1 1 1] Turret firing
  (Development|PrintString "Radius entered")
  (bind _asdhero_character (Utilities|Casting|CastToDHeroCharacter OtherActor))
  (Variables|Default|SetCharInRange true)
  (Variables|Default|SetProjectileTarget (Variables|/Script/Engine.Character|GetCapsuleComponent _asdhero_character))
  (Utilities|FlowControl|DoOnce false ; Gets rid of double fire on re-entry
    (:Completed
      (Utilities|Time|SetTimerbyEvent (delegate Custom|FireProjectile) 2.0 true)
      (bind _returnvalue (Game|SpawnActorfromClass "/Game/Blueprints/Actors/Turret_Projectile.Turret_Projectile_C" (Math|Conversions|ToTransform(Vector) (Transformation|GetWorldLocation (Variables|Default|GetProjectileSpawn))) "Undefined" 0 0))
      (Variables|/Game/Blueprints/Actors/Turret_Projectile.Turret_Projectile_C|SetProjectileTarget _returnvalue (Variables|Default|GetProjectileTarget)))))

(event OnComponentEndOverlap(AttackRadius)
  (params (OverlappedComponent :type Primitive%20Component%20Object%20Reference) (OtherActor :type Actor%20Object%20Reference) (OtherComp :type Primitive%20Component%20Object%20Reference) (OtherBodyIndex :type Integer))
  ;[1 1 1] Turret firing
  (Development|PrintString "Radius exited")
  (Utilities|Casting|CastToDHeroCharacter OtherActor)
  (Variables|Default|SetCharInRange false)
  (Utilities|Time|SetTimerbyEvent (delegate Custom|FireProjectile) 0.0)
  (Utilities|FlowControl|DoOnce false) ; enters at Reset
)

(event Custom|FireProjectile
  ;[1 1 1] Turret firing
  (bind _returnvalue (Game|SpawnActorfromClass "/Game/Blueprints/Actors/Turret_Projectile.Turret_Projectile_C" (Math|Conversions|ToTransform(Vector) (Transformation|GetWorldLocation (Variables|Default|GetProjectileSpawn))) "Undefined" 0 0))
  (Variables|/Game/Blueprints/Actors/Turret_Projectile.Turret_Projectile_C|SetProjectileTarget _returnvalue (Variables|Default|GetProjectileTarget)))

(event EventBeginPlay)

(event Collision|EventActorBeginOverlap
  (params (OtherActor :type Actor%20Object%20Reference)))

(fn ConstructionScript)