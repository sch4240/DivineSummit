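; Turret projectile actor that homes in on a target and damages the hero character.
; BeginPlay and every Tick assign ProjectileTarget as the homing target of its ProjectileMovement component.
; Overlapping a BP_HeroCharacter applies fixed damage and destroys the projectile, while other overlaps only print a failed-cast message.
; The Hit event is empty, and the construction script prints a spawn debug message.
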(event EventBeginPlay
  ;[1 1 1] Setting homing target
  (Variables|/Script/Engine.ProjectileMovementComponent|SetHomingTargetComponent (Variables|Default|GetProjectileMovement) (Variables|Default|GetProjectileTarget)))

(event EventTick
  (params (DeltaSeconds :type Float%20%28single-precision%29))
  ;[1 1 1] Setting homing target
  (Variables|/Script/Engine.ProjectileMovementComponent|SetHomingTargetComponent (Variables|Default|GetProjectileMovement) (Variables|Default|GetProjectileTarget)))

(event Collision|EventHit
  (params (MyComp :type Primitive%20Component%20Object%20Reference) (Other :type Actor%20Object%20Reference) (OtherComp :type Primitive%20Component%20Object%20Reference) (bSelfMoved :type Boolean) (HitLocation :type Vector :default "0, 0, 0") (HitNormal :type Vector :default "0, 0, 0") (NormalImpulse :type Vector :default "0, 0, 0") (Hit :type Hit%20Result%20Structure%20%28by%20ref%29))
  ;[1 1 1] Apply Damage
)

(event Collision|EventActorBeginOverlap
  (params (OtherActor :type Actor%20Object%20Reference))
  ;[1 1 1] Apply Damage
  (bind _asbp_hero_character (Utilities|Casting|CastToBP_HeroCharacter OtherActor)
    (:then
      (Game|Damage|ApplyDamage _asbp_hero_character 2e+01 0 0)
      (Actor|DestroyActor)
      (Development|PrintString "Projectile destroyed"))
    (:CastFailed
      (Development|PrintString "Cast failed"))))

(fn ConstructionScript
  (Development|PrintString "Projectile Spawned"))