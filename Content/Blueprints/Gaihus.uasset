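; Gaihus is an actor that reacts to the player character coming within range of its static mesh.
; A BeginPlay delay loop spawns a temporary PlaceholderPlant at the player's position, destroying it after a pause.
; A delayed Tick check drives the Move timeline, lerping the actor toward the player's halved world coordinates (not a midpoint) with an offset look-at rotation.
; Each update lerps from the current mesh transform and prints the alpha.
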(event Collision|EventActorBeginOverlap
  (params (OtherActor :type Actor%20Object%20Reference)))

(event EventTick
  (params (DeltaSeconds :type Float%20%28single-precision%29))
  (bind _staticmesh (Variables|Default|GetStaticMesh))
  (bind _returnvalue (Transformation|GetWorldLocation _staticmesh))
  (Utilities|FlowControl|Delay 1e+01 :!label _label)
  (if (<= (Math|Vector|Distance(Vector) (Transformation|GetWorldLocation (Variables|/Script/Engine.Character|GetMesh (Game|GetPlayerCharacter 0))) (Transformation|GetWorldLocation (Variables|Default|GetStaticMesh))) 1.5e+03)
    (bind _output_get (Variables|Default|SetLastLoc (/ (Transformation|GetWorldLocation (Variables|/Script/Engine.Character|GetMesh (Game|GetPlayerCharacter 0))) 2.0)))
    (bind _output_get_2 (Variables|Default|SetLastLocRot (Math|Rotator|CombineRotators (Math|Rotator|FindLookatRotation _returnvalue _output_get) "0,-90.000000, 0")))
    (bind _newtrack_1 (Timeline|Move PlayFromStart)
      (:Update
        (Development|PrintString (Utilities|String|ToString(Float) _newtrack_1))
        (Transformation|SetActorRotation (Math|Rotator|Lerp(Rotator) (Transformation|GetWorldRotation (Variables|Default|GetStaticMesh)) _output_get_2 _newtrack_1))
        (Transformation|SetActorLocation (Math|Vector|Lerp(Vector) _returnvalue _output_get _newtrack_1) false false)
        (Timeline|Move Play))
      (:Finished
        (goto _label)))))

(event EventBeginPlay
  (bind _returnvalue (Game|GetPlayerCharacter 0))
  (bind _mesh (Variables|/Script/Engine.Character|GetMesh _returnvalue))
  (bind _returnvalue_2 (Transformation|GetWorldLocation _mesh))
  (Utilities|FlowControl|Delay 5.0 :!label _label)
  (if (<= (Math|Vector|Distance(Vector) _returnvalue_2 (Transformation|GetWorldLocation (Variables|Default|GetStaticMesh))) 1.5e+03)
    (bind _returnvalue_3 (Game|SpawnActorfromClass "/Game/Blueprints/placeholderPlant.placeholderPlant_C" (Math|Conversions|ToTransform(Vector) _returnvalue_2) "Undefined" 0 0))
    (Utilities|FlowControl|Delay 5.0)
    (Actor|DestroyActor _returnvalue_3)
    (goto _label)
    (else
      (goto _label))))

(fn ConstructionScript)